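; Banana projectile actor that explodes with a radial impulse when its capsule hits something.
; On hit it stops its spin, turns on capsule physics and destroys the Banan component.
; A DoOnce gate then fires the RadialForce impulse, spawns an explosion particle with attached sound at that location, and destroys the actor after a short delay.
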(event `self.CapsuleCollision.OnComponentHit`
  (params (HitComponent :type "PrimitiveComponent Object Reference") (OtherActor :type "Actor Object Reference") (OtherComp :type "PrimitiveComponent Object Reference") (NormalImpulse :type "Vector Structure") (Hit :type "HitResult Structure (by ref)"))
  (bind _radialforce (`self.RadialForce`))
  ;[1 1 1] Banana Projectile
  (set `RotatingMovementComponent.RotationRate` (struct) (`self.RotatingMovement`))
  (`PrimitiveComponent.SetSimulatePhysics` (`self.CapsuleCollision`) true)
  (`ActorComponent.K2_DestroyComponent` (`self.Banan`))
  (`/Engine/EditorBlueprintResources/StandardMacros.DoOnce` false
    (:`Completed`
      (`RadialForceComponent.FireImpulse` _radialforce)
      (bind _returnvalue (`GameplayStatics.SpawnEmitterAtLocation` "/Game/StarterContent/Particles/P_Explosion.P_Explosion" (`SceneComponent.K2_GetComponentLocation` _radialforce)))
      (`GameplayStatics.SpawnSoundAttached` null _returnvalue)
      (`KismetSystemLibrary.Delay` 5.0)
      (`self.K2_DestroyActor`))))

(fn `UserConstructionScript`)
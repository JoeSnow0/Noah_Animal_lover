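; Pillar actor Blueprint that moves itself up and down in small timed steps.
; Tick, gated by an IsOverlappingActor check with no target actor given, reapplies the current yaw and waits on a variable Delay.
; A FlipFlop then alternates between hand-unrolled chains of local Z offsets and short Delays, one raising and one lowering the pillar without sweep.
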(event `self.ReceiveTick`
  (params (DeltaSeconds :type "Float (single-precision)"))
  (bind (_returnvalue_roll _returnvalue_pitch _returnvalue_yaw) (`KismetMathLibrary.BreakRotator` (`self.K2_GetActorRotation`)))
  ;[1 1 1] Make the pillers move up and down (Abraham Ohlsson)
  (if (not (`self.IsOverlappingActor` null))
    (`self.K2_SetActorRotation` (`KismetMathLibrary.MakeRotator` 0.0 0.0 _returnvalue_yaw))
    (`KismetSystemLibrary.Delay` (`self.Delay`))
    (`/Engine/EditorBlueprintResources/StandardMacros.FlipFlop`
      (:`A`
        (`self.K2_AddActorLocalOffset` (0.0 0.0 5.0))
        (`KismetSystemLibrary.Delay` 0.2)
        (`self.K2_AddActorLocalOffset` (0.0 0.0 5.0))
        (`KismetSystemLibrary.Delay` 0.2)
        (`self.K2_AddActorLocalOffset` (0.0 0.0 5.0))
        (`KismetSystemLibrary.Delay` 0.2)
        (`self.K2_AddActorLocalOffset` (0.0 0.0 5.0))
        (`KismetSystemLibrary.Delay` 0.2)
        (`self.K2_AddActorLocalOffset` (0.0 0.0 5.0))
        (`KismetSystemLibrary.Delay` 0.2)
        (`self.K2_AddActorLocalOffset` (0.0 0.0 5.0))
        (`KismetSystemLibrary.Delay` 0.2)
        (`self.K2_AddActorLocalOffset` (0.0 0.0 5.0))
        (`KismetSystemLibrary.Delay` 0.2)
        (`self.K2_AddActorLocalOffset` (0.0 0.0 5.0))
        (`KismetSystemLibrary.Delay` 0.2)
        (`self.K2_AddActorLocalOffset` (0.0 0.0 5.0))
        (`KismetSystemLibrary.Delay` 0.2)
        (`self.K2_AddActorLocalOffset` (0.0 0.0 5.0))
        (`KismetSystemLibrary.Delay` 0.2)
        (`self.K2_AddActorLocalOffset` (0.0 0.0 5.0))
        (`KismetSystemLibrary.Delay` 0.2)
        (`self.K2_AddActorLocalOffset` (0.0 0.0 5.0))
        (`KismetSystemLibrary.Delay` 0.2)
        (`self.K2_AddActorLocalOffset` (0.0 0.0 5.0))
        (`KismetSystemLibrary.Delay` 0.2)
        (`self.K2_AddActorLocalOffset` (0.0 0.0 5.0))
        (`KismetSystemLibrary.Delay` 0.2)
        (`self.K2_AddActorLocalOffset` (0.0 0.0 5.0))
        (`KismetSystemLibrary.Delay` 0.2)
        (`self.K2_AddActorLocalOffset` (0.0 0.0 5.0)))
      (:`B`
        (`self.K2_AddActorLocalOffset` (0.0 0.0 -5.0))
        (`KismetSystemLibrary.Delay` 0.2)
        (`self.K2_AddActorLocalOffset` (0.0 0.0 -5.0))
        (`KismetSystemLibrary.Delay` 0.2)
        (`self.K2_AddActorLocalOffset` (0.0 0.0 -5.0))
        (`KismetSystemLibrary.Delay` 0.2)
        (`self.K2_AddActorLocalOffset` (0.0 0.0 -5.0))
        (`KismetSystemLibrary.Delay` 0.2)
        (`self.K2_AddActorLocalOffset` (0.0 0.0 -5.0))
        (`KismetSystemLibrary.Delay` 0.2)
        (`self.K2_AddActorLocalOffset` (0.0 0.0 -5.0))
        (`KismetSystemLibrary.Delay` 0.2)
        (`self.K2_AddActorLocalOffset` (0.0 0.0 -5.0))
        (`KismetSystemLibrary.Delay` 0.2)
        (`self.K2_AddActorLocalOffset` (0.0 0.0 -5.0))
        (`KismetSystemLibrary.Delay` 0.2)
        (`self.K2_AddActorLocalOffset` (0.0 0.0 -5.0))
        (`KismetSystemLibrary.Delay` 0.2)
        (`self.K2_AddActorLocalOffset` (0.0 0.0 -5.0))
        (`KismetSystemLibrary.Delay` 0.2)
        (`self.K2_AddActorLocalOffset` (0.0 0.0 -5.0))
        (`KismetSystemLibrary.Delay` 0.2)
        (`self.K2_AddActorLocalOffset` (0.0 0.0 -5.0))
        (`KismetSystemLibrary.Delay` 0.2)
        (`self.K2_AddActorLocalOffset` (0.0 0.0 -5.0))
        (`KismetSystemLibrary.Delay` 0.2)
        (`self.K2_AddActorLocalOffset` (0.0 0.0 -5.0))
        (`KismetSystemLibrary.Delay` 0.2)
        (`self.K2_AddActorLocalOffset` (0.0 0.0 -5.0))
        (`KismetSystemLibrary.Delay` 0.2)
        (`self.K2_AddActorLocalOffset` (0.0 0.0 -5.0))))))

(fn `UserConstructionScript`)